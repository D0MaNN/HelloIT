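; BP_Walk is a pawn that uses AI movement to follow the target of a referenced changing-light object.
; On BeginPlay, FollowLight passes that target to the AIMove macro, provided the light reference is valid.
; AIMove wraps AIMoveTo in an optional loop, here re-issuing the move after a short delay on success or failure.
; A separate AIMoveToTarget event offers one-shot moves to an actor or location, but nothing here calls it.
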(event `self.ReceiveBeginPlay`
  (`self.FollowLight`))

(event `FollowLight`
  (bind _bp_changing_light (`self.BP Changing Light`)
    (:`then`
      (`self.AIMove` (0.0 0.0 0.0) (`/Engine/EngineMaterials/BP_ChangingLight.Target` _bp_changing_light) 10.0 true 2.0))
    (:`else`)))

(event `AIMoveToTarget`
  (params (Destination :type "Vector Structure") (TargetActor :type "Actor Object Reference") (AcceptanceRadius :type "Float (single-precision)"))
  (`/Engine/EditorBlueprintResources/StandardMacros.IsValid` TargetActor
    (:`Is Valid`
      (`|AIMoveTo` self (0.0 0.0 0.0) TargetActor AcceptanceRadius))
    (:`Is Not Valid`
      (`|AIMoveTo` self Destination null AcceptanceRadius))))

(fn `UserConstructionScript`)